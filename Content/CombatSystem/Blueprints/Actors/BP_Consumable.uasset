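; BP_Consumable is a limited-use item actor that modifies one of its owner's stats, with uses refilled to the maximum on BeginPlay.
; PerformItemAction has the owner play the use-item montage as a gameplay-tagged custom action, if uses remain.
; The separate ConsumeItem event decrements the count, reports it through the owner's health potion amount message and applies the change via BP_StatsComponent.
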(event `self.ReceiveBeginPlay`
  (`parent.ReceiveBeginPlay`)
  (set `self.CurrentNumberOfUses` (`self.MaxNumberOfUses`)))

(event `self.PerformItemAction`
  (if (> (`self.CurrentNumberOfUses`) 0)
    (message `/Game/CombatSystem/Blueprints/Interfaces/CombatBPI.PerformCustomAction` (`self.GetOwner`) (struct :`TagName` "Character.Action.Use Item") (struct :`TagName` "Character.State.General Action State") (`self.Use Item Montage`) 1.0 false)))

(event `ConsumeItem`
  (bind _result (`/Engine/EditorBlueprintResources/StandardMacros.DecrementInt` (`self.CurrentNumberOfUses`))
    (:`  `
      (message `/Game/CombatSystem/Blueprints/Interfaces/CombatBPI.UpdateHealthPotionAmount` (`self.GetOwner`) _result)
      (`/Game/CombatSystem/Blueprints/Components/BP_StatsComponent.ModifyCurrentStatValue` (`self.GetComponentByClass` (`self.GetOwner`) "/Game/CombatSystem/Blueprints/Components/BP_StatsComponent.BP_StatsComponent_C") (`self.Stat`) (`self.Modification Value`) (`self.Should Regenerate?`)))))

(fn `UserConstructionScript`
  (`parent.UserConstructionScript`))