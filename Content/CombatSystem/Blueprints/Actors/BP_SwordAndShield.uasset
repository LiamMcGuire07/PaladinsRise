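; BP_SwordAndShield is an equippable weapon that adds a shield to the inherited weapon behavior.
; It reattaches the shield mesh to the owning Character's mesh, using the hand socket when combat is enabled and the attach socket otherwise.
; Equip and combat-toggle overrides call their parent versions, then update that attachment.
; Equipping and unequipping also set the shield-equipped flag on the combat component.
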(event `self.ToggleWeaponCombat`
  (params (`bEnableCombat?` :type Boolean))
  (`parent.ToggleWeaponCombat` `bEnableCombat?`)
  (`self.AttachShield` (select `bool` `bEnableCombat?` :`false` (`self.ShieldAttachSocket`) :`true` (`self.ShieldHandSocket`))))

(fn `AttachShield`
  (params (`Attach Socket` :type Name))
  (`SceneComponent.K2_AttachToComponent` (`self.ShieldMesh`) (`Character.Mesh` (cast `Character` (`self.GetOwner`) :!pure true)) `Attach Socket` "KeepRelative" "KeepRelative" "KeepRelative" true))

(fn `OnEquipped`
  (`parent.OnEquipped`)
  (`self.AttachShield` (select `bool` (`/Game/CombatSystem/Blueprints/Components/BPC_CombatComponent.IsCombatEnabled?` (`self.CombatComponent`)) :`false` (`self.ShieldAttachSocket`) :`true` (`self.ShieldHandSocket`)))
  (`/Game/CombatSystem/Blueprints/Components/BPC_CombatComponent.SetShieldEquipped` (`self.CombatComponent`) true))

(fn `OnUnequipped`
  (`parent.OnUnequipped`)
  (`/Game/CombatSystem/Blueprints/Components/BPC_CombatComponent.SetShieldEquipped` (`self.CombatComponent`) false))

(fn `UserConstructionScript`
  (`parent.UserConstructionScript`))