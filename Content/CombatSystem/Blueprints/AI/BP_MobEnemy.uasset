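; BP_MobEnemy is a melee AI enemy that extends its parent with a weapon and a health bar shown only while targeted.
; A health bar widget reads StatsComponent, while RightWeaponCollisionComponent hits apply point damage from a current stat to actors that can receive it.
; Enabling combat plays a detection sound and snaps the weapon to its hand socket.
; On death, the weapon mesh switches to simulated physics.
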(event `self.ReceiveBeginPlay`
  (`parent.ReceiveBeginPlay`)
  (`/Game/CombatSystem/Blueprints/Components/BPC_CollisionComponent.SetCollisonMesh` (`self.RightWeaponCollisionComponent`) (`self.GetWeaponMesh`))
  (bind _returnvalue (`|CreateWidget` "/Game/CombatSystem/UI/Widgets/WB_HealthBar.WB_HealthBar_C" (`GameplayStatics.GetPlayerController` 0) (`self.StatsComponent`)))
  (`WidgetComponent.SetWidget` (`self.HealthBar`) _returnvalue))

(event `/Game/CombatSystem/Blueprints/Interfaces/TargetingBPI.OnTargeted`
  (params (`bIsTargeted?` :type Boolean))
  (`parent.OnTargeted` `bIsTargeted?`)
  (`SceneComponent.SetVisibility` (`self.HealthBar`) `bIsTargeted?` false))

(event `self.RightWeaponCollisionComponent.OnHit`
  (params (HitResult :type "HitResult Structure"))
  (bind (_bblockinghit _binitialoverlap _time _distance _location _impactpoint _normal _impactnormal _physmat _hitactor) (`GameplayStatics.BreakHitResult` HitResult))
  (bind _returnvalue (message `/Game/CombatSystem/Blueprints/Interfaces/CombatBPI.CanReceiveDamage` _hitactor))
  (if _returnvalue
    (`GameplayStatics.ApplyPointDamage` _hitactor (`/Game/CombatSystem/Blueprints/Components/BP_StatsComponent.GetCurrentStatValue` (`self.StatsComponent`) "NewEnumerator4") (`self.GetActorForwardVector`) HitResult (`self.GetController`) self "/Game/CombatSystem/Blueprints/DamageTypes/BP_AttackDamageType.BP_AttackDamageType_C")))

(event `SimulateWeaponPhysics`
  (bind _returnvalue (`self.GetWeaponMesh`))
  (`PrimitiveComponent.SetCollisionProfileName` _returnvalue "PhysicsActor" true)
  (`PrimitiveComponent.SetSimulatePhysics` _returnvalue true))

(event `self.PerformDeath`
  (`parent.PerformDeath`)
  (`self.SimulateWeaponPhysics`))

(event `self.CombatComponent.OnCombatToggled`
  (params (`bIsCombatEnabled?` :type Boolean))
  (if `bIsCombatEnabled?`
    (`GameplayStatics.PlaySoundAtLocation` (`self.Detection Sound`) (`self.K2_GetActorLocation`) (struct) 1.0 1.0 0.0 null null null null)
    (`SceneComponent.K2_AttachToComponent` (`self.GetWeaponMesh`) (`self.Mesh`) (select `bool` `bIsCombatEnabled?` :`false` (`self.Attach Socket Name`) :`true` (`self.Weapon Hand Socket`)) "SnapToTarget" "SnapToTarget" "SnapToTarget" true)))

(fn `GetWeapon`)

(fn `UserConstructionScript`
  (`parent.UserConstructionScript`))