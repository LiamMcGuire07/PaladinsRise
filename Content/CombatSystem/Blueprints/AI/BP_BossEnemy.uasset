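; Boss enemy Blueprint that extends a parent enemy class with an on-screen health bar and weapon hit damage.
; BeginPlay sets up the right weapon collision mesh and creates a WB_BossHealth widget bound to the StatsComponent.
; The bar shows while the boss has a valid target and hides on death.
; Hits from either weapon collision component apply stat-based point damage to actors able to receive it.
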(event `self.ReceiveBeginPlay`
  (`parent.ReceiveBeginPlay`)
  (`/Game/CombatSystem/Blueprints/Components/BPC_CollisionComponent.SetCollisonMesh` (`self.RightWeaponCollisionComponent`) null)
  (bind _returnvalue (`|CreateWidget` "/Game/CombatSystem/UI/Widgets/WB_BossHealth.WB_BossHealth_C" (`GameplayStatics.GetPlayerController` 0)))
  (bind _output_get (set `self.BossHealthUI` _returnvalue))
  (`/Game/CombatSystem/UI/Widgets/WB_BossHealth.Intialize` _output_get (`self.StatsComponent`))
  (`UserWidget.AddToViewport` (`self.BossHealthUI`) 0))

(event `SetBossHealthVisbility`
  (params (`IsVisible?` :type Boolean))
  (bind _bosshealthui (`self.BossHealthUI`)
    (:`then`
      (`Widget.SetVisibility` _bosshealthui (select `bool` (and `IsVisible?` (not (`/Game/CombatSystem/Blueprints/Components/BPC_StateManagerComponent.IsCurrentStateEqualToAny?` (`self.BPC_StateManagerComponent`) (struct :`GameplayTags` (struct :`(TagName` "Character.State.Dead")))))) :`false` "Hidden" :`true` "Visible" :!type "ESlateVisibility Enum")))
    (:`else`)))

(event `self.OnTargeted`
  (params (`bIsTargeted?` :type Boolean))
  (`parent.OnTargeted` `bIsTargeted?`))

(event `HitEvent`
  (params (HitResult :type "HitResult Structure"))
  (bind (_bblockinghit _binitialoverlap _time _distance _location _impactpoint _normal _impactnormal _physmat _hitactor) (`GameplayStatics.BreakHitResult` HitResult))
  (bind _returnvalue (message `/Game/CombatSystem/Blueprints/Interfaces/CombatBPI.CanReceiveDamage` _hitactor))
  (if _returnvalue
    (`GameplayStatics.ApplyPointDamage` _hitactor (`/Game/CombatSystem/Blueprints/Components/BP_StatsComponent.GetCurrentStatValue` (`self.StatsComponent`) "NewEnumerator4") (`self.GetActorForwardVector`) HitResult (`self.GetController`) self "/Game/CombatSystem/Blueprints/DamageTypes/BP_AttackDamageType.BP_AttackDamageType_C")))

(event `self.PerformDeath`
  (`parent.PerformDeath`)
  (`self.SetBossHealthVisbility` false))

(event `self.OnTargetSet`
  (params (NewTarget :type "Actor Object Reference"))
  (`parent.OnTargetSet` NewTarget)
  (`self.SetBossHealthVisbility` (`KismetSystemLibrary.IsValid` NewTarget)))

(event `self.LeftWeaponCollisionComponent.OnHit`
  (params (HitResult :type "HitResult Structure"))
  (`self.HitEvent` HitResult))

(event `self.RightWeaponCollisionComponent.OnHit`
  (params (HitResult :type "HitResult Structure"))
  (`self.HitEvent` HitResult))

(fn `UserConstructionScript`
  (`parent.UserConstructionScript`))