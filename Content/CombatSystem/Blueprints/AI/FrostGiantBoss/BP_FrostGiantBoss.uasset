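; Frost Giant boss character that plays an intro montage and drives the fight's music, phase change and end-of-game flow.
; The AI controller's first perception update swaps background music for phase-one music, and both weapon collision components use the boss mesh.
; Stat updates trigger phase two at half health, speeding up animations and switching tracks.
; At zero health it shows a thanks-for-playing widget, then a timer loads the main menu.
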(event `self.ReceiveBeginPlay`
  (bind _mesh (`self.Mesh`))
  (`parent.ReceiveBeginPlay`)
  (`ActorComponent.Activate` (`self.BackgroundMusic`) false)
  (bind _asbp_aicontroller (cast `/Game/CombatSystem/Blueprints/AI/BP_AIController` (`self.GetOwner`)))
  (set `self.Boss AIController` _asbp_aicontroller)
  ;[1 0 0] Start Boss Music once detected
  (add `AIPerceptionComponent.OnPerceptionUpdated` (`/Game/CombatSystem/Blueprints/AI/BP_AIController.AIPerception` (`self.Boss AIController`)) (delegate `StartBossMusic`))
  (`/Game/CombatSystem/Blueprints/Components/BPC_CollisionComponent.SetCollisonMesh` (`self.RightWeaponCollisionComponent`) _mesh)
  (`/Game/CombatSystem/Blueprints/Components/BPC_CollisionComponent.SetCollisonMesh` (`self.LeftWeaponCollisionComponent`) _mesh)
  (`self.PlayAnimMontage` "/Game/InfinityBladeAdversaries/Enemy/Enemy_Frost_Giant/Enemy_Frost_Giant_All_Animation/FrostGiant_Loop_CharacterIntro_Montage.FrostGiant_Loop_CharacterIntro_Montage"))

(event `StartBossMusic`
  (params (UpdatedActors :type "Array of Actor Object Reference (by ref)"))
  (bind _backgroundmusic (`self.BackgroundMusic`))
  ;[1 0 0] Start Boss Music once detected
  (`/Engine/EditorBlueprintResources/StandardMacros.DoOnce` false
    (:`Completed`
      (`ActorComponent.Activate` (`self.1stPhase`) false)
      (`AudioComponent.FadeOut` _backgroundmusic 1.0 0.0 "Linear")
      (`ActorComponent.Deactivate` _backgroundmusic))))

(event `self.StatsComponent.OnCurrentStatValueUpdated`
  (params (StatType :type "/Game/CombatSystem/Blueprints/Enums/E_Stats Enum" :default "NewEnumerator0") (Value :type "Float (double-precision)"))
  (bind _returnvalue (`|EnumEquality` StatType "NewEnumerator1"))
  ;[1 0 0] Phase Changes and Death
  (`|ExecutionSequence`
    (:`then_0`
      (if (and (`self.IsHalfHealth?` Value) _returnvalue)
        (`self.Phase 2 Start`)))
    (:`then_1`
      (if (and (<= Value 0.0) _returnvalue)
        (`AudioComponent.FadeOut` (`self.2ndPhase`) 1.0 0.0 "Linear")
        (`ActorComponent.Activate` (`self.BackgroundMusic`) false)
        (bind _returnvalue_2 (`|CreateWidget` "/Game/CombatSystem/UI/Widgets/WB_ThanksForPlaying.WB_ThanksForPlaying_C"))
        (`UserWidget.AddToViewport` _returnvalue_2 0)
        (`KismetSystemLibrary.K2_SetTimerDelegate` (delegate `BackToMainMenu`) (`self.CountdownToMainMenu`))))))

(event `BackToMainMenu`
  ;[1 0 0] Phase Changes and Death
  (`Widget.RemoveFromParent` (stale `self.StatsComponent.OnCurrentStatValueUpdated` _returnvalue_2))
  (`GameplayStatics.OpenLevelBySoftObjectPtr` "/Game/InfinityBladeIceLands/Maps/FrozenCoveMainMenu.FrozenCoveMainMenu"))

(fn `IsHalfHealth?`
  (params (HP :type "Float (double-precision)"))
  (returns (ReturnValue :type Boolean))
  (return (<= HP (* 0.5 (`/Game/CombatSystem/Blueprints/Components/BP_StatsComponent.GetMaxStatValue` (`self.StatsComponent`) "NewEnumerator1")))))

(fn `Phase 2 Start`
  (bind _1stphase (`self.1stPhase`))
  (set `SkeletalMeshComponent.GlobalAnimRateScale` 1.5 (`self.Mesh`))
  (`AudioComponent.FadeOut` _1stphase 1.0 0.0 "Linear")
  (`ActorComponent.Deactivate` _1stphase)
  (`ActorComponent.Activate` (`self.2ndPhase`) false))

(fn `UserConstructionScript`
  (`parent.UserConstructionScript`))